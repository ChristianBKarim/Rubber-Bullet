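; BP_Bullet is a physics-driven projectile that launches along its Arrow's forward vector at BulletSpeed on spawn.
; Tick snaps it back to X = 0 when it drifts past a small tolerance, confining flight to the YZ plane.
; Tick also sets its rotation through a look-at toward a vector built from the velocity's CalculateDirection value.
; A timer destroys the bullet after a fixed lifetime.
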(event `self.ReceiveBeginPlay`
  (`PrimitiveComponent.SetPhysicsLinearVelocity` (`self.Bullet`) (* (* (`SceneComponent.GetForwardVector` (`self.Arrow`)) (`self.BulletSpeed`)) 100.0) false "None")
  (`self.SetActorTickEnabled` true)
  (`KismetSystemLibrary.K2_SetTimerDelegate` (delegate `DestroyBulletDelay`) 10.0))

(event `DestroyBulletDelay`
  (`self.K2_DestroyActor`))

(event `self.ReceiveTick`
  (params (DeltaSeconds :type "Float (single-precision)"))
  (bind _bullet (`self.Bullet`))
  (bind (_returnvalue_x _returnvalue_y _returnvalue_z) (`KismetMathLibrary.BreakVector` (`SceneComponent.K2_GetComponentLocation` (`self.Bullet`))))
  (`|ExecutionSequence`
    (:`then_0`
      (if (or (> _returnvalue_x 2.0) (< _returnvalue_x -2.0))
        (`SceneComponent.K2_SetWorldLocation` (`self.Bullet`) (`KismetMathLibrary.MakeVector` 0.0 _returnvalue_y _returnvalue_z) false false)))
    (:`then_1`
      (`SceneComponent.K2_SetWorldRotation` (`self.Bullet`) (`KismetMathLibrary.FindLookAtRotation` (`self.K2_GetActorLocation`) (`KismetMathLibrary.Conv_DoubleToVector` (`KismetAnimationLibrary.CalculateDirection` (`SceneComponent.GetComponentVelocity` _bullet) (`SceneComponent.K2_GetComponentRotation` _bullet)))) false false))))

(fn `UserConstructionScript`)