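; Player controller for an orthographic character game that handles the fixed camera view, mouse aim input and firing.
; On BeginPlay it switches the view to a level CameraActor, looping back until one is found, then caches the character and passes itself to its animation Blueprint.
; Vertical mouse movement accumulates into a clamped, sensitivity-scaled position value.
; Left click makes the character spawn a projectile, gated by a timer-reset cooldown.
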(event `self.ReceiveBeginPlay`
  (bind _returnvalue (`GameplayStatics.GetActorOfClass` "/Script/Engine.CameraActor" :!label _label))
  (`/Engine/EditorBlueprintResources/StandardMacros.IsValid` _returnvalue
    (:`Is Valid`
      (`self.SetViewTargetWithBlend` (`GameplayStatics.GetPlayerController` 0) _returnvalue 0.0 "VTBlend_Linear" 0.0 false)
      (bind _asbp_orthographic_character (cast `/Game/Characters/Player/BP_Orthographic_Character` (`GameplayStatics.GetPlayerCharacter` 0)))
      (bind _output_get (set `self.OrthoCharacter` _asbp_orthographic_character))
      (bind _asabp_unarmed (cast `/Game/Characters/Mannequins/Anims/Unarmed/ABP_Unarmed` (`SkeletalMeshComponent.GetAnimInstance` (`Character.Mesh` _output_get))))
      (set `/Game/Characters/Mannequins/Anims/Unarmed/ABP_Unarmed.ControllerRef` self _asabp_unarmed))
    (:`Is Not Valid`
      (goto _label))))

(event `InputAxisKey|MouseY`
  (params (AxisValue :type "Float (single-precision)"))
  (set `self.MouseYPosition` (`KismetMathLibrary.FClamp` (+ (* (`self.Sensitivity`) AxisValue) (`self.MouseYPosition`)) -50.0 50.0)))

(event `Key|LeftMouseButton`
  (params (Key :type "Key Structure"))
  (:`Pressed`
    (if (not (`self.bOnCooldown`))
      (`/Game/Characters/Player/BP_Orthographic_Character.SpawnProjectile` (`self.OrthoCharacter`))
      (set `self.bOnCooldown` true)
      (`KismetSystemLibrary.K2_SetTimerDelegate` (delegate `ResetbOnCooldown`) 1.0))))

(event `ResetbOnCooldown`
  (set `self.bOnCooldown` false))

(fn `UserConstructionScript`)