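; BP_TestBullet is a test projectile that launches on spawn and is held near the world X = 0 plane.
; BeginPlay sets the Bullet component's physics linear velocity along the Arrow's forward vector, scaled from BulletSpeed, then enables Tick.
; Tick acts as a manual plane constraint, snapping the bullet's X back to zero whenever it drifts outside a small tolerance, keeping Y and Z.
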(event `self.ReceiveBeginPlay`
  (`PrimitiveComponent.SetPhysicsLinearVelocity` (`self.Bullet`) (* (* (`SceneComponent.GetForwardVector` (`self.Arrow`)) (`self.BulletSpeed`)) 100.0) false "None")
  (`self.SetActorTickEnabled` true))

(event `self.ReceiveTick`
  (params (DeltaSeconds :type "Float (single-precision)"))
  (bind (_returnvalue_x _returnvalue_y _returnvalue_z) (`KismetMathLibrary.BreakVector` (`SceneComponent.K2_GetComponentLocation` (`self.Bullet`))))
  (`|ExecutionSequence`
    (:`then_0`
      (if (or (> _returnvalue_x 10.0) (< _returnvalue_x -10.0))
        (`SceneComponent.K2_SetWorldLocation` (`self.Bullet`) (`KismetMathLibrary.MakeVector` 0.0 _returnvalue_y _returnvalue_z) false false)))))

(fn `UserConstructionScript`)