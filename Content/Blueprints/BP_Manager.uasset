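; BP_Manager is a level manager that shows the win screen when the enemy dies.
; On BeginPlay it finds a single BP_Enemy, binds to its Dead event, sets game-only input and hides the mouse cursor.
; OnEnemyDead creates a WB_YouWin widget, passes it the last-level flag and the level to load, and adds it to the viewport.
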(event `self.ReceiveBeginPlay`
  (bind _returnvalue (`GameplayStatics.GetPlayerController` 0))
  (bind _returnvalue_2 (`GameplayStatics.GetActorOfClass` "/Game/Blueprints/BP_Enemy.BP_Enemy_C"))
  (add `/Game/Blueprints/BP_Enemy.Dead` _returnvalue_2 (`|CreateDelegate` :!event `OnEnemyDead`))
  (`WidgetBlueprintLibrary.SetInputMode_GameOnly` _returnvalue)
  (set `PlayerController.bShowMouseCursor` false _returnvalue))

(event `OnEnemyDead`
  (bind _returnvalue (`|CreateWidget` "/Game/Blueprints/WB_YouWin.WB_YouWin_C" null (`self.LastLevel?`) (`self.LevelToLoad`)))
  (`UserWidget.AddToViewport` _returnvalue 0))

(fn `UserConstructionScript`)