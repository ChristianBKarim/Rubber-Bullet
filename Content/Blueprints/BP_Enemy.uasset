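; Enemy actor that dies from a single hit by a BP_Bullet.
; On that hit it turns on mesh physics, destroys its capsule and pushes the mesh with the hit's normal impulse for a ragdoll-style death.
; It also calls its Dead dispatcher, plays a 2D hurt sound and starts a short timer that destroys the actor.
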(event `self.ReceiveHit`
  (params (MyComp :type "PrimitiveComponent Object Reference") (Other :type "Actor Object Reference") (OtherComp :type "PrimitiveComponent Object Reference") (bSelfMoved :type Boolean) (HitLocation :type "Vector Structure") (HitNormal :type "Vector Structure") (NormalImpulse :type "Vector Structure") (Hit :type "HitResult Structure (by ref)"))
  (cast `/Game/Blueprints/BP_Bullet` Other)
  (`PrimitiveComponent.SetSimulatePhysics` (`self.Mesh`) true)
  (`ActorComponent.K2_DestroyComponent` (`self.CapsuleComponent`))
  (`KismetSystemLibrary.K2_SetTimerDelegate` (delegate `EnemyDied`) 3.0)
  (`self.Dead`)
  (`PrimitiveComponent.AddImpulse` (`self.Mesh`) NormalImpulse "None" false)
  (`GameplayStatics.PlaySound2D` "/Game/SFX/hurt.hurt" 1.0 1.0 0.0 null null))

(event `EnemyDied`
  (`self.K2_DestroyActor`))

(fn `UserConstructionScript`)