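; BP_Orthographic_Character is a player character Blueprint that fires BP_Bullet projectiles on left mouse click, except in the LVL_MainMenu level.
; Each shot spawns a bullet at Arrow1's world location along its forward vector and plays a 2D gun sound.
; An OnCooldown flag limits the fire rate, with a timer event clearing it after a short delay.
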(event `SpawnProjectile`
  (bind _arrow1 (`self.Arrow1`))
  (`|SpawnActorFromClass` "/Game/Blueprints/BP_Bullet.BP_Bullet_C" (`KismetMathLibrary.MakeTransform` (`SceneComponent.K2_GetComponentLocation` _arrow1) (`KismetMathLibrary.Conv_VectorToRotator` (`SceneComponent.GetForwardVector` _arrow1))) "Undefined" "MultiplyWithRoot" null null))

(event `Key|LeftMouseButton`
  (params (Key :type "Key Structure"))
  (:`Pressed`
    (bind _returnvalue (`GameplayStatics.GetCurrentLevelName` true))
    (if (`KismetStringLibrary.NotEqual_StrStr` _returnvalue "LVL_MainMenu")
      (if (not (`self.bOnCooldown`))
        (`self.SpawnProjectile`)
        (set `self.bOnCooldown` true)
        (`KismetSystemLibrary.K2_SetTimerDelegate` (delegate `ResetbOnCooldown`) 1.0)
        (`GameplayStatics.PlaySound2D` "/Game/SFX/gun.gun" 1.0 1.0 0.0 null null)))))

(event `ResetbOnCooldown`
  (set `self.bOnCooldown` false))

(fn `UserConstructionScript`)